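; Actor Blueprint that moves a Uranus component along an elliptical spline path, apparently as its orbit.
; Each tick it advances a distance by Speed and sets the component's relative location from the spline's local transform at that distance, keeping its scale.
; When IsLooping is set, the distance resets to zero after passing the spline's length, so the motion repeats.
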(event `self.ReceiveTick`
  (params (DeltaSeconds :type "Float (single-precision)"))
  (bind _uranus (`self.Uranus`))
  (bind _returnvalue_location (`KismetMathLibrary.BreakTransform` (`SplineComponent.GetTransformAtDistanceAlongSpline` (`self.Uranus_Ellipse`) (`self.Distance`) "Local" false)))
  (set `self.Distance` (+ (* DeltaSeconds (`self.Speed`)) (`self.Distance`)))
  (`SceneComponent.K2_SetRelativeTransform` _uranus (`KismetMathLibrary.MakeTransform` _returnvalue_location (struct) (`SceneComponent.RelativeScale3D` _uranus)) false false)
  (if (`self.isLooping`)
    (if (> (`self.Distance`) (`SplineComponent.GetSplineLength` (`self.Uranus_Ellipse`)))
      (set `self.Distance` 0.0))))

(fn `UserConstructionScript`)