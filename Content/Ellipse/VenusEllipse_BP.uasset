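; Actor Blueprint that moves a Venus component along an elliptical spline, as an orbit path.
; Each Tick advances DistanceVenus by SpeedVenus scaled by delta time and places Venus at that local-space spline location, keeping its scale.
; When IsLoopingVenus is set, the distance resets to zero once it exceeds the spline length, restarting the lap.
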(event `self.ReceiveTick`
  (params (DeltaSeconds :type "Float (single-precision)"))
  (bind _venus (`self.Venus`))
  (bind _returnvalue_location (`KismetMathLibrary.BreakTransform` (`SplineComponent.GetTransformAtDistanceAlongSpline` (`self.Spline`) (`self.Distance_Venus`) "Local" false)))
  (set `self.Distance_Venus` (+ (* DeltaSeconds (`self.Speed_Venus`)) (`self.Distance_Venus`)))
  (`SceneComponent.K2_SetRelativeTransform` _venus (`KismetMathLibrary.MakeTransform` _returnvalue_location (struct) (`SceneComponent.RelativeScale3D` _venus)) false false)
  (if (`self.isLooping_Venus`)
    (if (> (`self.Distance_Venus`) (`SplineComponent.GetSplineLength` (`self.Spline`)))
      (set `self.Distance_Venus` 0.0))))

(fn `UserConstructionScript`)