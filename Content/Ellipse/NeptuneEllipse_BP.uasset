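; Actor Blueprint that moves a Neptune component along an elliptical spline path, acting as the planet's orbit.
; Each Tick adds Speed times delta time to a running Distance and sets Neptune's relative location from the local-space spline transform at that distance.
; Rotation is not taken from the spline, and the existing scale is kept.
; When IsLooping is set, Distance resets to zero after passing the spline's length.
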(event `self.ReceiveTick`
  (params (DeltaSeconds :type "Float (single-precision)"))
  (bind _neptune (`self.Neptune`))
  (bind _returnvalue_location (`KismetMathLibrary.BreakTransform` (`SplineComponent.GetTransformAtDistanceAlongSpline` (`self.Neptune_Ellipse`) (`self.Distance`) "Local" false)))
  (set `self.Distance` (+ (* DeltaSeconds (`self.Speed`)) (`self.Distance`)))
  (`SceneComponent.K2_SetRelativeTransform` _neptune (`KismetMathLibrary.MakeTransform` _returnvalue_location (struct) (`SceneComponent.RelativeScale3D` _neptune)) false false)
  (if (`self.isLooping`)
    (if (> (`self.Distance`) (`SplineComponent.GetSplineLength` (`self.Neptune_Ellipse`)))
      (set `self.Distance` 0.0))))

(fn `UserConstructionScript`)