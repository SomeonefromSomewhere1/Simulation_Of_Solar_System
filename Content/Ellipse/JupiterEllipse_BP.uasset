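; Actor Blueprint that moves a Jupiter component along an elliptical spline path, apparently as a planetary orbit.
; Each Tick advances a distance by Speed and delta time, then places Jupiter at that spline point in local space, keeping its scale but not following spline rotation.
; When IsLooping is set, the distance resets to zero past the spline's end.
; The spline component is named MarsEllipse despite driving Jupiter.
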(event `self.ReceiveTick`
  (params (DeltaSeconds :type "Float (single-precision)"))
  (bind _jupiter (`self.Jupiter`))
  (bind _returnvalue_location (`KismetMathLibrary.BreakTransform` (`SplineComponent.GetTransformAtDistanceAlongSpline` (`self.Mars_Ellipse`) (`self.Distance`) "Local" false)))
  (set `self.Distance` (+ (* DeltaSeconds (`self.Speed`)) (`self.Distance`)))
  (`SceneComponent.K2_SetRelativeTransform` _jupiter (`KismetMathLibrary.MakeTransform` _returnvalue_location (struct) (`SceneComponent.RelativeScale3D` _jupiter)) false false)
  (if (`self.isLooping`)
    (if (> (`self.Distance`) (`SplineComponent.GetSplineLength` (`self.Mars_Ellipse`)))
      (set `self.Distance` 0.0))))

(fn `UserConstructionScript`)